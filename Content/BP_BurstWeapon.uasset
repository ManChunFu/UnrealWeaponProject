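; Burst weapon Blueprint that a character auto-equips on mesh overlap when holding no other weapon.
; FireMode component starts and stops firing; each Attack, unless suspended, spends one round and fires BP_Projectile with inaccuracy from the Recoil component.
; Alt attack press and release both call Scope zoom on the holder's first-person camera.
; Reload refills via the Ammo component and also changes the fire mode.
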(event `self.StartAltAttack`
  (bind _asfirst_person_character (cast `/Game/FirstPersonCPP/Blueprints/FirstPersonCharacter` (`self.Holder`) :!label _label))
  (`ScopeComponent.Zoom` (`self.Scope`) (`UnrealWeaponProjectCharacter.FirstPersonCameraComponent` _asfirst_person_character)))

(event `self.StopAltAttack`
  (goto _label))

(event `self.StartAttack`
  (`FireModeComponent.Start` (`self.FireMode1`)))

(event `self.StopAttack`
  (`FireModeComponent.Stop` (`self.FireMode1`)))

(event `self.Attack`
  (if (== (`self.SuspendedFromAttack`) 0)
    (bind _returnvalue (`AmmoComponent.DecreaseAmmo` (`self.Ammo`) 1))
    (if _returnvalue
      (`RecoilComponent.AddRecoil` (`self.Recoil`) 0.0 0.0)
      (bind (_actualrecoilx _actualrecoily) (`RecoilComponent.DoRecoil` (`self.Recoil`)))
      (`ProjectileComponent.FireProjectile` :`self` (`self.Projectile`) :`ProjectileClass` "/Game/BP_Projectile.BP_Projectile_C" :`Owner` (`self.Holder`) :`InaccuracyZ` _actualrecoilx :`InaccuracyY` _actualrecoily))))

(event `self.Reload`
  (`AmmoComponent.Reload` (`self.Ammo`))
  (`FireModeComponent.ChangeFireMode` (`self.FireMode1`)))

(event `self.WeaponMesh.OnComponentBeginOverlap`
  (params (OverlappedComponent :type "PrimitiveComponent Object Reference") (OtherActor :type "Actor Object Reference") (OtherComp :type "PrimitiveComponent Object Reference") (OtherBodyIndex :type Integer) (bFromSweep :type Boolean) (SweepResult :type "HitResult Structure (by ref)"))
  (bind _asunreal_weapon_project_character (cast `UnrealWeaponProjectCharacter` OtherActor))
  (if (not (`KismetSystemLibrary.IsValid` (`UnrealWeaponProjectCharacter.EquippedWeapon` _asunreal_weapon_project_character)))
    (`UnrealWeaponProjectCharacter.EquipWeapon` _asunreal_weapon_project_character self)))

(fn `UserConstructionScript`)