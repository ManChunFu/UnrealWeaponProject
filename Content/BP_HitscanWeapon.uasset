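; BP_HitscanWeapon is a weapon that fires hitscan attacks from the first-person camera of its holder.
; Start and stop attack events drive a FireMode component through AutoFire and Stop.
; Attack runs only while SuspendedFromAttack is zero and the Holder casts to FirstPersonCharacter.
; It passes the camera's location and forward vector to WeaponHitScan for the trace, with the debug line enabled.
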(event `self.StartAttacking`
  (`FireModeComponent.AutoFire` (`self.FireMode`)))

(event `self.StopAttacking`
  (`FireModeComponent.Stop` (`self.FireMode`)))

(event `self.Attack`
  (if (== (`self.SuspendedFromAttack`) 0)
    (bind _asfirst_person_character (cast `/Game/FirstPersonCPP/Blueprints/FirstPersonCharacter` (`self.Holder`)))
    (bind _firstpersoncameracomponent (`UnrealWeaponProjectCharacter.FirstPersonCameraComponent` _asfirst_person_character))
    (`WeaponHitScanComponent.OnAttack` (`self.WeaponHitScan`) (`SceneComponent.K2_GetComponentLocation` _firstpersoncameracomponent) (`SceneComponent.GetForwardVector` _firstpersoncameracomponent) true)))

(fn `UserConstructionScript`)