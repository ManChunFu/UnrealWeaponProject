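; BP_WeaponTwo is a weapon Blueprint that fires laser projectiles for the player character.
; Its Attack event runs the parent attack, spawns a BP_Laser through a projectile component owned by player 0, then triggers a camera shake on that character.
; An overlap on the weapon mesh auto-equips it to a character that has no weapon equipped.
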(event `self.Attack`
  (bind _returnvalue (`GameplayStatics.GetPlayerCharacter` 0))
  (`parent.Attack`)
  (`ProjectileComponent.FireProjectile` :`self` (`self.Projectile`) :`ProjectileClass` "/Game/BP_Laser.BP_Laser_C" :`Owner` _returnvalue)
  (bind _asunreal_weapon_project_character (cast `UnrealWeaponProjectCharacter` _returnvalue))
  (`CameraShakeComponent.DoCameraShake` (`self.CameraShake`) _asunreal_weapon_project_character null))

(event `self.WeaponMesh.OnComponentBeginOverlap`
  (params (OverlappedComponent :type "PrimitiveComponent Object Reference") (OtherActor :type "Actor Object Reference") (OtherComp :type "PrimitiveComponent Object Reference") (OtherBodyIndex :type Integer) (bFromSweep :type Boolean) (SweepResult :type "HitResult Structure (by ref)"))
  (bind _asunreal_weapon_project_character (cast `UnrealWeaponProjectCharacter` OtherActor))
  (if (not (`KismetSystemLibrary.IsValid` (`UnrealWeaponProjectCharacter.EquippedWeapon` _asunreal_weapon_project_character)))
    (`UnrealWeaponProjectCharacter.EquipWeapon` _asunreal_weapon_project_character self)))

(fn `UserConstructionScript`)